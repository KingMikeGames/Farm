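; Player character with an ice-slide movement ability, an upward-thrust control and a dash, which also creates the HUD on BeginPlay.
; Holding right mouse switches to Flying and loops a timer that traces down, stamps short-lived ice decals and repositions one reused BP_IcePlatform at the hit.
; Tick applies ReverseGravity while Space is held, otherwise FlyingGravity when flying.
; Left Shift applies an impulse along the arrow component's forward vector.
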(event `IcePath`
  (bind _returnvalue (`self.K2_GetActorLocation`))
  (bind (_outhit _returnvalue_2) (`KismetSystemLibrary.LineTraceSingle` _returnvalue (- _returnvalue (0.0 0.0 120.0)) "TraceTypeQuery1"))
  (if _returnvalue_2
    (bind (_bblockinghit _binitialoverlap _time _location _impactpoint _normal) (`GameplayStatics.BreakHitResult` _outhit))
    (`GameplayStatics.SpawnDecalAtLocation` "/Game/Materials/Decal/IcePath.IcePath" (20.0 100.0 100.0) _impactpoint (`KismetMathLibrary.MakeRotFromX` _normal) 1.5)
    (set `self.IsSliding` true)
    (bind _outactors (`GameplayStatics.GetAllActorsOfClass` "/Game/Blueprint/BP_IcePlatform.BP_IcePlatform_C"))
    (if (== (`KismetArrayLibrary.Array_Length` _outactors) 0)
      (`|SpawnActorFromClass` "/Game/Blueprint/BP_IcePlatform.BP_IcePlatform_C" (`KismetMathLibrary.MakeTransform` _impactpoint (struct) (2.0 2.0 2.0)) "Undefined" "OverrideRootScale")
      (else
        (`self.K2_SetActorLocation` (`KismetArrayLibrary.Array_Get` _outactors) _impactpoint false true)))
    (else
      (set `self.IsSliding` false))))

(event `self.OnLanded`
  (params (Hit :type "HitResult Structure (by ref)"))
  (if (> (`PlayerController.GetInputKeyTimeDown` (`GameplayStatics.GetPlayerController` 0) "RightMouseButton") 0.0)
    (`CharacterMovementComponent.SetMovementMode` (`self.CharacterMovement`) "MOVE_Flying" 0 :!label _label)
    (bind _returnvalue (`KismetSystemLibrary.K2_SetTimerDelegate` (delegate `IcePath`) 0.016 true))
    (set `self.Timer` _returnvalue)))

(event `Key|RightMouseButton`
  (params (Key :type "Key Structure" :default "AnyKey"))
  (:`Pressed`
    (goto _label))
  (:`Released`
    (`CharacterMovementComponent.SetMovementMode` (`self.CharacterMovement`) "MOVE_Walking" 0)
    (`KismetSystemLibrary.K2_ClearAndInvalidateTimerHandle` (`self.Timer`))
    (set `self.IsSliding` false)))

(event `self.ReceiveBeginPlay`
  (bind _returnvalue (`|CreateWidget` "/Game/UI/Hud.Hud_C"))
  (`UserWidget.AddToViewport` _returnvalue 0))

(event `self.ReceiveTick`
  (params (DeltaSeconds :type "Float (single-precision)"))
  (bind _charactermovement (`self.CharacterMovement`))
  (`|ExecutionSequence`
    (:`then_0`
      (if (> (`PlayerController.GetInputKeyTimeDown` (`GameplayStatics.GetPlayerController` 0) "SpaceBar") 0.0)
        (`CharacterMovementComponent.AddForce` _charactermovement (`self.ReverseGravity`))
        (elif (`NavMovementComponent.IsFlying` _charactermovement)
          (`CharacterMovementComponent.AddForce` _charactermovement (`self.FlyingGravity`)))))))

(event `Key|LeftShift`
  (params (Key :type "Key Structure" :default "AnyKey"))
  (:`Pressed`
    (`CharacterMovementComponent.AddImpulse` (`self.CharacterMovement`) (* (`SceneComponent.GetForwardVector` (`self.ArrowComponent`)) 70000.0) false)))

(fn `UserConstructionScript`)